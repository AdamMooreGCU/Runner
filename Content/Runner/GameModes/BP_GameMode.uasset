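; Game mode for a runner game that builds the floor track and handles the player's death.
; On BeginPlay it spawns a run of BP_FloorTile actors, chaining them by storing each new tile's spawn transform for the next one.
; PlayerHitObstacle passes through a DoOnce, so the OnDeath dispatcher and a leftover debug print fire only on the first hit.
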(event `self.ReceiveBeginPlay`
  (for _ (range 30)
    (`self.SpawnFloorTile`)))

(event `PlayerHitObstacle`
  (`/Engine/EditorBlueprintResources/StandardMacros.DoOnce` false
    (:`Completed`
      (`self.OnDeath`)
      (`KismetSystemLibrary.PrintString` "Hello"))))

(fn `SpawnFloorTile`
  (bind _returnvalue (`|SpawnActorFromClass` "/Game/Runner/Blueprints/BP_FloorTile.BP_FloorTile_C" (`self.TileSpawnTransform`) "Undefined" "MultiplyWithRoot" null null))
  (bind _tilespawntransform (`/Game/Runner/Blueprints/BP_FloorTile.GetTileSpawnTransform` _returnvalue))
  (set `self.TileSpawnTransform` _tilespawntransform)
  (return))

(fn `UserConstructionScript`)