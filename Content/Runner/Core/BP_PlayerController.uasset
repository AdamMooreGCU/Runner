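; Player controller for the runner game that turns left and right input into lane-style moves on the runner character.
; On BeginPlay it adds the runner Enhanced Input mapping context and binds to the game mode's death event.
; Move left and right actions forward to the possessed BP_RunnerCharacter.
; When death fires, the controller disables its own input.
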(event `self.ReceiveBeginPlay`
  (`EnhancedInputSubsystemInterface.AddMappingContext` (subsystem `EnhancedInputLocalPlayerSubsystem`) "/Game/Runner/Input/IMC_Runner.IMC_Runner" 0 (struct))
  (add `/Game/Runner/GameModes/BP_GameMode.OnDeath` (cast `/Game/Runner/GameModes/BP_GameMode` (`GameplayStatics.GetGameMode`) :!pure true) (`|CreateDelegate` :!event `OnDeath`)))

(event `EnhancedInput|/Game/Runner/Input/InputActions/IA_MoveLeft`
  (params (ActionValue :type Boolean) (ElapsedSeconds :type "Float (double-precision)") (TriggeredSeconds :type "Float (double-precision)") (InputAction :type "InputAction Object Reference" :default "/Game/Runner/Input/InputActions/IA_MoveLeft.IA_MoveLeft"))
  (:`Started`
    (bind _asbp_runner_character (cast `/Game/Runner/Core/BP_RunnerCharacter` (`self.K2_GetPawn`)))
    (`/Game/Runner/Core/BP_RunnerCharacter.MoveLeft` _asbp_runner_character)))

(event `EnhancedInput|/Game/Runner/Input/InputActions/IA_MoveRight`
  (params (ActionValue :type Boolean) (ElapsedSeconds :type "Float (double-precision)") (TriggeredSeconds :type "Float (double-precision)") (InputAction :type "InputAction Object Reference" :default "/Game/Runner/Input/InputActions/IA_MoveRight.IA_MoveRight"))
  (:`Started`
    (bind _asbp_runner_character (cast `/Game/Runner/Core/BP_RunnerCharacter` (`self.K2_GetPawn`)))
    (`/Game/Runner/Core/BP_RunnerCharacter.MoveRight` _asbp_runner_character)))

(event `OnDeath`
  (`self.DisableInput` self))

(fn `UserConstructionScript`)