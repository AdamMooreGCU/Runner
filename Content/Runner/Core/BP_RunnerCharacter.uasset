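; Player character for a runner game that moves forward automatically along world X and switches between three lanes.
; Tick feeds constant forward movement input while Alive.
; MoveLeft and MoveRight check the current lane, apply an instant swept sideways offset of MoveDistance, then update the lane state.
; BeginPlay binds to the game mode's OnDeath, which ragdolls the mesh and clears Alive to stop the forward input.
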(event `self.ReceiveBeginPlay`
  (add `/Game/Runner/GameModes/BP_GameMode.OnDeath` (cast `/Game/Runner/GameModes/BP_GameMode` (`GameplayStatics.GetGameMode`) :!pure true) (`|CreateDelegate` :!event `OnDeath`)))

(event `self.ReceiveTick`
  (params (DeltaSeconds :type "Float (single-precision)"))
  (if (`self.bAlive`)
    (`PawnMovementComponent.AddInputVector` (`self.CharacterMovement`) (1.0 0.0 0.0) false)))

(event `OnDeath`
  (`PrimitiveComponent.SetSimulatePhysics` (`self.Mesh`) true)
  (`PrimitiveComponent.SetCollisionProfileName` (`self.Mesh`) "Ragdoll" true)
  (set `self.bAlive` false))

(fn `MoveLeft`
  (switch `/Game/Runner/Core/ELane` (`self.CurrentLane`)
    (:`NewEnumerator1`
      _)
    (:`NewEnumerator2`
      _))
  (`MovementComponent.K2_MoveUpdatedComponent` :`self` (`self.CharacterMovement`) :`Delta` (`KismetMathLibrary.MakeVector` 0.0 (* (`self.MoveDistance`) -1.0)))
  (switch `/Game/Runner/Core/ELane` (`self.CurrentLane`)
    (:`NewEnumerator1`
      (set `self.CurrentLane` "NewEnumerator0"))
    (:`NewEnumerator2`
      (set `self.CurrentLane` "NewEnumerator1"))))

(fn `MoveRight`
  (switch `/Game/Runner/Core/ELane` (`self.CurrentLane`)
    (:`NewEnumerator0`
      _)
    (:`NewEnumerator1`
      _))
  (`MovementComponent.K2_MoveUpdatedComponent` :`self` (`self.CharacterMovement`) :`Delta` (`KismetMathLibrary.MakeVector` 0.0 (`self.MoveDistance`)))
  (switch `/Game/Runner/Core/ELane` (`self.CurrentLane`)
    (:`NewEnumerator0`
      (set `self.CurrentLane` "NewEnumerator1"))
    (:`NewEnumerator1`
      (set `self.CurrentLane` "NewEnumerator2"))))

(fn `UserConstructionScript`)