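; BP_FloorTile is a floor segment for a runner game that places one BP_Obstacle in a random left, center or right lane on BeginPlay.
; The obstacle is a runtime child actor component positioned at that lane's marker transform.
; When the runner character overlaps TriggerBox, the tile asks BP_GameMode to spawn another tile, then destroys itself immediately.
; GetTileSpawnTransform exposes the TileSpawnPoint world transform, while SpawnCollectable is an empty stub.
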(event `self.ReceiveBeginPlay`
  (`self.SpawnObstacle`))

(event `self.TriggerBox.OnComponentBeginOverlap`
  (params (OverlappedComponent :type "PrimitiveComponent Object Reference") (OtherActor :type "Actor Object Reference") (OtherComp :type "PrimitiveComponent Object Reference") (OtherBodyIndex :type Integer) (bFromSweep :type Boolean) (SweepResult :type "HitResult Structure (by ref)"))
  (cast `/Game/Runner/Core/BP_RunnerCharacter` OtherActor)
  (`/Game/Runner/GameModes/BP_GameMode.SpawnFloorTile` (cast `/Game/Runner/GameModes/BP_GameMode` (`GameplayStatics.GetGameMode`) :!pure true))
  (`self.K2_DestroyActor`))

(fn `GetTileSpawnTransform`
  (returns (TileSpawnTransform :type "Transform Structure"))
  (return (`SceneComponent.K2_GetComponentToWorld` (`self.TileSpawnPoint`))))

(fn `SpawnCollectable`)

(fn `SpawnObstacle`
  (bind _output_get (set `self.ObstacleLane` (cast `/Game/Runner/Core/ELane` (`KismetMathLibrary.Conv_IntToByte` (`KismetMathLibrary.RandomIntegerInRange` 0 2)))))
  (switch `/Game/Runner/Core/ELane` _output_get
    (:`NewEnumerator0`
      (bind _returnvalue (`AddComponent|NODE_AddChildActorComponent-1` :`RelativeTransform` (`SceneComponent.GetRelativeTransform` (`self.LeftObstacle`))))
      (`ChildActorComponent.SetChildActorClass` _returnvalue "/Game/Runner/Blueprints/BP_Obstacle.BP_Obstacle_C")
      (return))
    (:`NewEnumerator1`
      (bind _returnvalue_2 (`AddComponent|NODE_AddChildActorComponent-2` :`RelativeTransform` (`SceneComponent.GetRelativeTransform` (`self.CenterObstacle`))))
      (`ChildActorComponent.SetChildActorClass` _returnvalue_2 "/Game/Runner/Blueprints/BP_Obstacle.BP_Obstacle_C")
      (return))
    (:`NewEnumerator2`
      (bind _returnvalue_3 (`AddComponent|NODE_AddChildActorComponent-3` :`RelativeTransform` (`SceneComponent.GetRelativeTransform` (`self.RightObstacle`))))
      (`ChildActorComponent.SetChildActorClass` _returnvalue_3 "/Game/Runner/Blueprints/BP_Obstacle.BP_Obstacle_C")
      (return))))

(fn `UserConstructionScript`)